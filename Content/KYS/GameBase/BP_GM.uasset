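; Game mode BP_GM that scatters players at spawn and holds an unfinished game-over flow.
; On player restart, it moves the BP_Player pawn to a random reachable navmesh point within a wide radius of a PlayerStart.
; CheckWinner uses a validity check to set IsGameOver once and call EndGame.
; EndGame and GetMostKillPlayer have no working logic, only empty bodies or disconnected winner and kill-leader lookups.
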(event `self.K2_OnRestartPlayer`
  (params (NewPlayer :type "Controller Object Reference"))
  ; 월드에대한 모든 이관이 끝난후 호출
  (bind _asbp_player (cast `/Game/KYS/BP_Player` (`Controller.K2_GetPawn` NewPlayer)))
  (`self.MoveAtRandomLocation` _asbp_player))

(fn `CheckWinner`
  (if (not (`self.IsGameOver`))
    (`/Engine/EditorBlueprintResources/StandardMacros.IsValid` null
      (:`Is Valid`
        (`|ExecutionSequence`
          (:`then_0`
            (set `self.IsGameOver` true))
          (:`then_1`
            (`self.EndGame`)))))))

(fn `EndGame`)

(fn `GetMostKillPlayer`
  (returns (PlayerState :type "Object Object Reference")))

(fn `MoveAtRandomLocation`
  (params (InActor :type "Actor Object Reference"))
  (bind _returnvalue (`GameplayStatics.GetActorOfClass` "/Script/Engine.PlayerStart"))
  (bind (_randomlocation _returnvalue_2) (`NavigationSystemV1.K2_GetRandomReachablePointInRadius` (`self.K2_GetActorLocation` _returnvalue) 50000.0 null null))
  (if _returnvalue_2
    (`self.K2_SetActorLocation` (`local.InActor`) _randomlocation false false)))

(fn `UserConstructionScript`)