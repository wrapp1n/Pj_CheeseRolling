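; Lobby game mode that names joining players, holds match settings and moves the lobby to the game level through seamless server travel.
; PostLogin gives each BP_LobbyPlayerState a numbered "User" nickname from an incrementing index.
; SaveConfig stores the level name locally and writes a clamped max player count to BP_GameInstance.
; TryStartGame waits briefly, then runs a ServerTravel console command built from the saved level name.
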(event `self.ReceiveBeginPlay`
  (set `self.bUseSeamlessTravel` true))

(event `TryStartGame`
  (`KismetSystemLibrary.Delay` 1.0)
  (`KismetSystemLibrary.ExecuteConsoleCommand` (`KismetStringLibrary.Concat_StrStr` "ServerTravel " (`self.LevelName`)) null))

(event `self.K2_PostLogin`
  (params (NewPlayer :type "PlayerController Object Reference"))
  ; Set Nickname
  (bind _asbp_lobby_player_state (cast `/Game/KYS/Lobby/BP_LobbyPlayerState` (`Controller.PlayerState` NewPlayer)))
  (bind _result (`/Engine/EditorBlueprintResources/StandardMacros.IncrementInt` (`self.NicknameIndex`))
    (:`  `
      (set `/Game/KYS/Lobby/BP_LobbyPlayerState.Nickname` (`|FormatText` "User{0}" _result) _asbp_lobby_player_state))))

(fn `SaveConfig`
  (params (InLevelName :type String) (InMaxPlayerConunt :type Integer))
  (locals (BPGameInstance :type "/Game/KYS/GameBase/BP_GameInstance Object Reference"))
  (`|ExecutionSequence`
    (:`then_0`
      (set `self.LevelName` (`local.InLevelName`)))
    (:`then_1`
      (bind _asbp_game_instance (cast `/Game/KYS/GameBase/BP_GameInstance` (`GameplayStatics.GetGameInstance`)))
      (set `local.BPGameInstance` _asbp_game_instance))
    (:`then_2`
      (set `/Game/KYS/GameBase/BP_GameInstance.MaxPlayerCount` (`KismetMathLibrary.Clamp` (`local.InMaxPlayerConunt`) 2 10) (`local.BPGameInstance`)))))

(fn `UserConstructionScript`)