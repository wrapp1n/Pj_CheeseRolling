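; BP_Cheese is a physics-driven round cheese that keeps itself moving and spinning.
; BeginPlay offsets the center of mass, sets a maximum angular velocity and starts two looping timers, leaving Tick unused.
; CheckSpeed pops a slow cheese upward with a random sideways impulse that ignores mass.
; Spin rapidly applies torque around the horizontal axis perpendicular to travel, derived by crossing velocity direction with up.
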(event `self.ReceiveBeginPlay`
  (`PrimitiveComponent.SetCenterOfMass` (`self.cheese_round`) (0.3 0.5 0.2) "None")
  (`PrimitiveComponent.SetPhysicsMaxAngularVelocityInDegrees` (`self.cheese_round`) 700.0 false "None")
  (`KismetSystemLibrary.K2_SetTimer` null "CheckSpeed" 0.5 true)
  (`KismetSystemLibrary.K2_SetTimer` null "Spin" 0.01 true))

(event `self.ReceiveTick`
  (params (DeltaSeconds :type "Float (single-precision)")))

(fn `CheckSpeed`
  (bind _returnvalue (`PrimitiveComponent.GetPhysicsLinearVelocity` (`self.cheese_round`) "None"))
  (if (< (`KismetMathLibrary.VSize` _returnvalue) 100.0)
    (`PrimitiveComponent.AddImpulse` (`self.cheese_round`) (`KismetMathLibrary.MakeVector` (`KismetMathLibrary.RandomFloatInRange` -300.0 300.0) (`KismetMathLibrary.RandomFloatInRange` -300.0 300.0) 400.0) "None" true)))

(fn `Spin`
  (bind _returnvalue (`PrimitiveComponent.GetPhysicsLinearVelocity` (`self.cheese_round`) "None"))
  (`PrimitiveComponent.AddTorqueInDegrees` (`self.cheese_round`) (* (`KismetMathLibrary.Cross_VectorVector` (`KismetMathLibrary.Vector_Normal2D` _returnvalue 1.0) (0.0 0.0 1.0)) 10000.0) "None" true))

(fn `UserConstructionScript`)